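; BP_PacMan is the player-controlled Pac-Man, moved freely in the XY plane by axis input.
; The MoveX and MoveY axes each set one component of CurrentVelocity from clamped input scaled by Speed, so diagonal movement is not normalized.
; Tick applies any non-zero velocity times delta time through SetActorLocation without sweep, so movement does not stop at collisions.
; BeginPlay, Initialize and the construction script are empty.
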(event `self.ReceiveBeginPlay`)

(event `self.ReceiveTick`
  (params (DeltaSeconds :type "Float (single-precision)"))
  (if (not (`KismetMathLibrary.Vector_IsZero` (`self.CurrentVelocity`)))
    (bind _newlocation (`self.GetNewLocation` DeltaSeconds))
    (`self.K2_SetActorLocation` _newlocation)))

(event `InputAxis|MoveX`
  (params (AxisValue :type "Float (single-precision)"))
  (`self.Move_XAxis` AxisValue))

(event `InputAxis|MoveY`
  (params (AxisValue :type "Float (single-precision)"))
  (`self.Move_YAxis` AxisValue))

(fn `GetNewLocation`
  (params (DeltaSeconds :type "Float (double-precision)"))
  (returns (NewLocation :type "Vector Structure"))
  (bind _output_get (set `self.NewLocation` (+ (`self.K2_GetActorLocation`) (* (`self.CurrentVelocity`) DeltaSeconds))))
  (return _output_get))

(fn `Initialize`)

(fn `Move_XAxis`
  (params (AxisValue :type "Float (double-precision)"))
  (bind (_currentvelocity_x _currentvelocity_y _currentvelocity_z) (`KismetMathLibrary.BreakVector` (`self.CurrentVelocity`)))
  (set `self.CurrentVelocity` (`KismetMathLibrary.MakeVector` (* (`KismetMathLibrary.FClamp` AxisValue -1.0) (`self.Speed`)) _currentvelocity_y _currentvelocity_z)))

(fn `Move_YAxis`
  (params (AxisValue :type "Float (double-precision)"))
  (bind (_currentvelocity_x _currentvelocity_y _currentvelocity_z) (`KismetMathLibrary.BreakVector` (`self.CurrentVelocity`)))
  (set `self.CurrentVelocity` (`KismetMathLibrary.MakeVector` _currentvelocity_x (* (`KismetMathLibrary.FClamp` AxisValue -1.0) (`self.Speed`)) _currentvelocity_z)))

(fn `UserConstructionScript`)